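; BP_DynamicCameraSystem is a follow-camera actor that trails player character 0 with smoothed movement and rotation.
; Each Tick it builds a target from the character's forward, right and up vectors scaled by Offset, and a rotation combining RotOffset with the character's rotation.
; It lerps toward both by SmoothSpeed times delta time, rotating along the shortest path.
; BeginPlay caches the BP_Player_Dino actor in Player, which Tick does not use.
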(event `self.ReceiveBeginPlay`
  (bind _returnvalue (`GameplayStatics.GetActorOfClass` "/Game/Characters/Dino/Dino_Walking/BP_Player_Dino.BP_Player_Dino_C"))
  (set `self.Player` _returnvalue))

(event `self.ReceiveTick`
  (params (DeltaSeconds :type "Float (single-precision)"))
  (`self.K2_SetActorLocation` (`KismetMathLibrary.VLerp` (`self.K2_GetActorLocation`) (+ (+ (* (`self.GetActorForwardVector` (`GameplayStatics.GetPlayerCharacter` 0)) (.y (`self.Offset`))) (* (`self.GetActorRightVector` (`GameplayStatics.GetPlayerCharacter` 0)) (.x (`self.Offset`))) (* (`self.GetActorUpVector` (`GameplayStatics.GetPlayerCharacter` 0)) (.z (`self.Offset`)))) (`self.K2_GetActorLocation` (`GameplayStatics.GetPlayerCharacter` 0))) (* (`self.smoothSpeed`) (`GameplayStatics.GetWorldDeltaSeconds`))))
  (`self.K2_SetActorRotation` (`KismetMathLibrary.RLerp` (`self.K2_GetActorRotation`) (`KismetMathLibrary.ComposeRotators` (`self.rotOffset`) (`self.K2_GetActorRotation` (`GameplayStatics.GetPlayerCharacter` 0))) (* (`self.smoothSpeed`) (`GameplayStatics.GetWorldDeltaSeconds`)) true)))

(fn `UserConstructionScript`)