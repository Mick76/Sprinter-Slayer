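; Playable or AI-driven dinosaur character for a bone-grabbing game, with movement gated by CanStart.
; Each tick it traces from the jaw to the Bone, ignoring other dinos, snapping a takeable bone onto the jaw when close.
; At mid range the trace updates Steering, which AI dinos follow as movement input.
; StartDash boosts walk speed until a timer expires; the patrol behavior tree and SteeringCalc are unused.
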(event `self.ReceiveBeginPlay`
  (set `self.defaultWalkSpeed` (`CharacterMovementComponent.MaxWalkSpeed` (`self.CharacterMovement`)))
  (bind _outactors (`GameplayStatics.GetAllActorsOfClass` "BP_Player_Dino_C"))
  (set `self.otherPlayers` _outactors))

(event `InputAxis|MoveForward`
  (params (AxisValue :type "Float (single-precision)"))
  (if (`self.canStart`)
    (`self.AddMovementInput` (`self.GetActorForwardVector`) AxisValue)))

(event `InputAxis|MoveRight`
  (params (AxisValue :type "Float (single-precision)"))
  (if (`self.canStart`)
    (`self.AddMovementInput` (`self.GetActorRightVector`) AxisValue)))

(event `self.ReceiveTick`
  (params (DeltaSeconds :type "Float (single-precision)"))
  (if (`self.canStart`)
    (`self.CheckBone`)
    (if (`self.isAI`)
      (`self.AddMovementInput` (`self.Steering`)))
    (if (`self.Dashing`)
      (bind _output_get (set `self.dashTimeCounter` (+ (`self.dashTimeCounter`) (`GameplayStatics.GetWorldDeltaSeconds`))))
      (`/Engine/EditorBlueprintResources/StandardMacros.CompareFloat` _output_get (`self.dashTime`)
        (:`>`
          (set `self.dashTimeCounter` 0.0)
          (set `self.Dashing` false)
          (set `CharacterMovementComponent.MaxWalkSpeed` (`self.defaultWalkSpeed`) (`self.CharacterMovement`)))))))

(fn `CheckBone`
  (bind _returnvalue (`SceneComponent.GetSocketLocation` (`self.Mesh`) "jaw_tip"))
  (bind _returnvalue_2 (`self.K2_GetActorLocation` (`self.bone`)))
  (bind _outhit (`KismetSystemLibrary.LineTraceSingle` _returnvalue _returnvalue_2 "TraceTypeQuery1" false (`self.otherPlayers`)))
  (bind (_bblockinghit _binitialoverlap _time _distance _location _impactpoint _normal _impactnormal _physmat _hitactor) (`GameplayStatics.BreakHitResult` _outhit))
  (bind _asbp_bone (cast `/Game/Characters/Dino/Dino_Walking/BP_Bone` _hitactor))
  (`/Engine/EditorBlueprintResources/StandardMacros.CompareFloat` _distance 150.0
    (:`>`
      (set `self.hasBone` false)
      (`/Engine/EditorBlueprintResources/StandardMacros.CompareFloat` _distance 800.0
        (:`<`
          (set `self.Steering` (`KismetMathLibrary.Normal` (- _returnvalue_2 _returnvalue))))))
    (:`<`
      (if (`/Game/Characters/Dino/Dino_Walking/BP_Bone.canBeTaken` _asbp_bone)
        (if (not (`self.hasBone`))
          (set `/Game/Characters/Dino/Dino_Walking/BP_Bone.Taken` true _asbp_bone)
          (set `self.hasBone` true)
          (set `/Game/Characters/Dino/Dino_Walking/BP_Bone.currentDino` self _asbp_bone)
          (`self.K2_AttachToComponent` _asbp_bone (`self.Mesh`) "jaw_tip" "SnapToTarget" "SnapToTarget" "SnapToTarget" true)
          (`self.K2_SetActorRelativeRotation` _asbp_bone (struct :`Pitch` 90.0 :`Yaw` 90.0) false false)
          (set `/Game/Characters/Dino/Dino_Walking/BP_Bone.coolDownTimeCounter` 0.0 _asbp_bone)
          (`AudioComponent.Play` (`/Game/Characters/Dino/Dino_Walking/BP_Bone.audio` _asbp_bone) 0.0)
          (set `/Game/Characters/Dino/Dino_Walking/BP_Bone.coolingDown` true _asbp_bone))))))

(fn `StartDash`
  (if (`self.Dashing`)
    (set `self.dashTimeCounter` 0.0)
    (else
      (set `self.Dashing` true)
      (set `CharacterMovementComponent.MaxWalkSpeed` (+ 500.0 (`self.defaultWalkSpeed`)) (`self.CharacterMovement`)))))

(fn `UserConstructionScript`)