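; BP_Bone is a movable bone Character that can be taken and has a cooldown before it can be taken again.
; Once CanStart is set, Tick disables movement while Taken, otherwise moves it along the Steering vector.
; While CoolingDown, Tick accumulates delta time and restores CanBeTaken when CoolDown is exceeded.
; The RandomPatrol behavior tree launch, StartDash speed change and steering calculation are disconnected.
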(event `self.ReceiveBeginPlay`
  ;[1 1 1] Start behavior tree to make Dino's wander around.
)

(event `self.ReceiveTick`
  (params (DeltaSeconds :type "Float (single-precision)"))
  (if (`self.canStart`)
    (if (`self.Taken`)
      (`ActorComponent.SetActive` (`self.CharacterMovement`) false false)
      (else
        (`ActorComponent.SetActive` (`self.CharacterMovement`) true false)
        (`self.AddMovementInput` (`self.Steering`))))
    (if (`self.coolingDown`)
      (bind _output_get (set `self.coolDownTimeCounter` (+ (`self.coolDownTimeCounter`) (`GameplayStatics.GetWorldDeltaSeconds`))))
      (`/Engine/EditorBlueprintResources/StandardMacros.CompareFloat` _output_get (`self.coolDown`)
        (:`>`
          (set `self.canBeTaken` true)
          (set `self.coolDownTimeCounter` 0.0)
          (set `self.coolingDown` false))
        (:`<`
          (set `self.canBeTaken` false))))))

(fn `StartDash`
  (if true
    _))

(fn `UserConstructionScript`)